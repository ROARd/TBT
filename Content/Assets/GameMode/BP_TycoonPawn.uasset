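; BP_TycoonPawn is the tycoon game's pawn, moved by the Forward and Right input axes.
; Each axis event offsets DefaultSceneRoot in world space along that component's own forward or right vector, scaled by the axis value and a fixed speed.
; Movement skips sweep collision and is not scaled by delta time, so its speed depends on frame rate.
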(event Input|AxisEvents|InputAxisForward
  (params (AxisValue :type Float%20%28single-precision%29))
  (bind _defaultsceneroot (Variables|Default|GetDefaultSceneRoot))
  (Transformation|AddWorldOffset _defaultsceneroot (* (Math|Vector|GetForwardVector _defaultsceneroot) (* AxisValue 1e+01)) false false))

(event Input|AxisEvents|InputAxisRight
  (params (AxisValue :type Float%20%28single-precision%29))
  (bind _defaultsceneroot (Variables|Default|GetDefaultSceneRoot))
  (Transformation|AddWorldOffset _defaultsceneroot (* (Math|Vector|GetRightVector _defaultsceneroot) (* AxisValue 1e+01)) false false))

(fn ConstructionScript)