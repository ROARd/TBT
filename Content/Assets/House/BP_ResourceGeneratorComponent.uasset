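; Actor component that generates a house resource over time up to a maximum capacity, configured through Init.
; Tick accumulates time and adds one unit whenever the generate interval elapses, carrying over the remainder, then fires Filled and stops ticking at capacity.
; Ticking is disabled at BeginPlay and starts on Purge, which broadcasts the gathered amount and resets it to zero.
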(event Custom|Init
  (params (MaxCapacity :type Integer) (GenerateInterval :type Float%20%28single-precision%29))
  (Variables|Default|SetResourceMaxCapacity MaxCapacity)
  (Variables|Default|SetResourceGenerateInterval GenerateInterval))

(event Custom|Purge
  (Components|Tick|SetComponentTickEnabled true)
  (Default|CallPurged (Variables|Default|GetResourceAggregated))
  (Variables|Default|SetResourceAggregated 0))

(event EventBeginPlay
  (Components|Tick|SetComponentTickEnabled false))

(event EventTick
  (params (DeltaSeconds :type Float%20%28single-precision%29))
  (bind _resourcemaxcapacity (Variables|Default|GetResourceMaxCapacity))
  (bind _output_get (Variables|Default|SetResourceGenerateTimer (+ DeltaSeconds (Variables|Default|GetResourceGenerateTimer))))
  (if (> (Math|Float|Truncate (/ _output_get (Variables|Default|GetResourceGenerateInterval))) 0)
    (Variables|Default|SetResourceGenerateTimer (Math|Float|%(Float) (Variables|Default|GetResourceGenerateTimer) (Variables|Default|GetResourceGenerateInterval)))
    (bind _output_get_2 (Variables|Default|SetResourceAggregated (Math|Integer|Clamp(Integer) (+ 1 (Variables|Default|GetResourceAggregated)) 0 _resourcemaxcapacity)))
    (if (== _output_get_2 _resourcemaxcapacity)
      (Default|CallFilled)
      (Components|Tick|SetComponentTickEnabled false))))