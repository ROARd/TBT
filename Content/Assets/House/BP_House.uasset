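; House actor for a tycoon game that is built over time, then generates resources for the player.
; HouseStruct configures a construction component and a resource generator component.
; Completing construction swaps the mesh from constructing to constructed material and enables generator ticking; purged amounts go to player 0's TycoonPlayerState.
; It exposes a widget anchor, offset on BeginPlay by the mesh's lower Z bound.
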(event Custom|OnConstructed
  ;[1 1 1] ConstructionComponent bindings
  (Rendering|Material|SetMaterial (Variables|Default|GetStaticMesh) 0 (Variables|Default|GetConstructedMat))
  (Components|Tick|SetComponentTickEnabled (Variables|Default|GetBP_ResourceGenerator) true))

(event Custom|OnHousePurged
  (params (Amount :type Integer))
  ;[1 1 1] ResourceGenerator bindings
  (Class|TycoonPlayerState|AddResource (.AsTycoon%20Player%20State (Utilities|Casting|CastToTycoonPlayerState (Variables|/Script/Engine.Controller|GetPlayerState (Game|GetPlayerController 0)))) Amount))

(event EventBeginPlay
  (bind _housestruct (Variables|Default|GetHouseStruct))
  (bind _staticmesh (Variables|Default|GetStaticMesh))
  (Utilities|FlowControl|Sequence
    (:then_0
      ;[1 1 1] Init
      (Default|Init (Variables|Default|GetBP_ConstructionComponent) (.buildtime _housestruct))
      (Default|Init (Variables|Default|GetBP_ResourceGenerator) (.resourcemaxcapacity _housestruct) (.resourcegenerateinterval _housestruct))
      (Rendering|Material|SetMaterial _staticmesh 0 (Variables|Default|GetConstructingMat))
      (Transformation|AddLocalOffset (Variables|Default|GetWidgetPoint) (Math|Vector|MakeVector 0.0 0.0 (.Z (Math|Vector|BreakVector (.Min (Components|StaticMesh|GetLocalBounds _staticmesh))))) false false))
    (:then_1
      ;[1 1 1] ConstructionComponent bindings
      (EventDispatchers|AssignConstructed (Variables|Default|GetBP_ConstructionComponent) (delegate Custom|OnConstructed)))
    (:then_2
      ;[1 1 1] ResourceGenerator bindings
      (EventDispatchers|BindEventtoPurged (Variables|Default|GetBP_ResourceGenerator) (delegate Custom|OnHousePurged)))))

(fn ConstructionScript)

(fn GetWidgetPlacement
  (return (Variables|Default|GetWidgetPoint)))